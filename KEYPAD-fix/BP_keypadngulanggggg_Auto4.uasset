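; Interactable passcode keypad that registers itself with the BP_contoh player while they overlap its box.
; Interacting blends the view to its camera, enables mouse clicks, shows dot placeholders and links child-actor buttons back to the keypad for digit, backspace and confirm input.
; A correct code turns the lamp green, returns the camera and removes the interaction box.
; A wrong code shows "Try again", blocks digit entry, then re-initialises after a delay.
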(event `self.Boxcollision.OnComponentBeginOverlap`
  (params (OverlappedComponent :type "PrimitiveComponent Object Reference") (OtherActor :type "Actor Object Reference") (OtherComp :type "PrimitiveComponent Object Reference") (OtherBodyIndex :type Integer) (bFromSweep :type Boolean) (SweepResult :type "HitResult Structure (by ref)"))
  ;[1 1 1] on overlap events, set player references
  (message `/Game/KEYPAD-fix/bp_interface.interact_area_entered` OtherActor)
  (if (== OtherActor (`GameplayStatics.GetPlayerPawn` 0))
    (bind _asbp_contoh (cast `/Game/ThirdPerson/Blueprints/BP_contoh` OtherActor))
    (set `/Game/ThirdPerson/Blueprints/BP_contoh.Keypad Interact Actor` self _asbp_contoh)
    (set `self.player ref` _asbp_contoh)))

(event `self.Boxcollision.OnComponentEndOverlap`
  (params (OverlappedComponent :type "PrimitiveComponent Object Reference") (OtherActor :type "Actor Object Reference") (OtherComp :type "PrimitiveComponent Object Reference") (OtherBodyIndex :type Integer))
  ;[1 1 1] on overlap events, set player references
  (message `/Game/KEYPAD-fix/bp_interface.interact_area_exited` OtherActor)
  (if (== OtherActor (`GameplayStatics.GetPlayerPawn` 0))
    (bind _asbp_contoh (cast `/Game/ThirdPerson/Blueprints/BP_contoh` OtherActor))
    (set `/Game/ThirdPerson/Blueprints/BP_contoh.Keypad Interact Actor` null _asbp_contoh)
    (set `self.player ref` null)))

(event `On interacted`
  (bind _returnvalue (`GameplayStatics.GetPlayerController` 0))
  (bind _entered_code (`self.entered code`))
  (bind _returnvalue_2 (`KismetStringLibrary.GetSubstring` "...." 0 (`KismetStringLibrary.Len` (`self.kwypad code`))))
  ;[1 1 1] ini supaya kl player interact kamera bisa switch smoothly
  (`PlayerController.SetViewTargetWithBlend` (`GameplayStatics.GetPlayerController` 0) (`ActorComponent.GetOwner` (`self.Camera`)) 0.4 "VTBlend_Linear" 0.0 false)
  (bind _output_get (set `PlayerController.bShowMouseCursor` true _returnvalue :!label _label))
  (bind _output_get_2 (set `PlayerController.bEnableClickEvents` _output_get _returnvalue))
  (set `PlayerController.bEnableMouseOverEvents` _output_get_2 _returnvalue)
  (`TextRenderComponent.K2_SetText` _entered_code (`KismetSystemLibrary.MakeLiteralText` (`KismetTextLibrary.Conv_StringToText` _returnvalue_2)))
  (`TextRenderComponent.SetTextRenderColor` _entered_code (make `Color` 200 200 200 255))
  (`KismetSystemLibrary.PrintString` _returnvalue_2)
  (bind _output_get_3 (set `self.Buttons Array` (`|MakeArray` (`self.1`) (`self.2`) (`self.3`) (`self.4`) (`self.5`) (`self.6`) (`self.7`) (`self.8`) (`self.9`) (`self.0`) (`self.hapus`) (`self.enter`))))
  (for _array_element _output_get_3
    (bind _askeyyyyyyangka (cast `/Game/KEYPAD-fix/keyyyyyyangka` (`ChildActorComponent.ChildActor` _array_element)))
    (set `/Game/KEYPAD-fix/keyyyyyyangka.Keypad actor ref` self _askeyyyyyyangka)))

(event `Initiate`
  ;[1 1 1] ini supaya kl player interact kamera bisa switch smoothly
  (goto _label))

(event `Button Entered`
  (params (Value :type Text) (Confirmed :type Boolean) (backspace :type Boolean))
  (bind _entered_code (`self.entered code`))
  ;[1 1 1] button dipencet
  (if Confirmed
    (`self.on confirmed`)
    (elif backspace
      (`self.backspace`)
      (elif (`self.canEnter`)
        (`TextRenderComponent.K2_SetText` _entered_code (`KismetTextLibrary.Conv_StringToText` (`KismetStringLibrary.Replace` (`KismetTextLibrary.Conv_TextToString` (`TextRenderComponent.Text` (`self.entered code`))) (`KismetStringLibrary.GetSubstring` "...." 0 (`KismetStringLibrary.Len` (`self.kwypad code`))))))
        (`TextRenderComponent.K2_SetText` _entered_code (`KismetTextLibrary.Conv_StringToText` (`KismetStringLibrary.Concat_StrStr` (`KismetTextLibrary.Conv_TextToString` (`TextRenderComponent.Text` (`self.entered code`))) (`KismetTextLibrary.Conv_TextToString` Value))))
        (`TextRenderComponent.SetTextRenderColor` (`self.entered code`) (make `Color` 255 255 255 255))))))

(event `backspace`
  (bind _entered_code (`self.entered code`))
  (bind _returnvalue (`KismetTextLibrary.Conv_TextToString` (`TextRenderComponent.Text` _entered_code)))
  ;[1 1 1] stlah pass dimasukin
  ;;[1 1 1] backspace
  (`TextRenderComponent.K2_SetText` _entered_code (`KismetTextLibrary.Conv_StringToText` (`KismetStringLibrary.GetSubstring` _returnvalue 0 (- (`KismetStringLibrary.Len` _returnvalue) 1)))))

(event `on confirmed`
  (bind _returnvalue (`GameplayStatics.GetPlayerController` 0))
  (bind _returnvalue_2 (`GameplayStatics.GetPlayerController` 0))
  (bind _entered_code (`self.entered code`))
  (bind _entered_code_2 (`self.entered code`))
  ;[1 1 1] stlah pass dimasukin
  ;;[1 1 1] passcode bnr, berubah warna, reset kamera. gbs di interact lg
  (if (`KismetStringLibrary.EqualEqual_StrStr` (`self.kwypad code`) (`KismetTextLibrary.Conv_TextToString` (`TextRenderComponent.Text` (`self.entered code`))))
    (`|ExecutionSequence`
      (:`then_0`
        (`TextRenderComponent.K2_SetText` _entered_code_2 "Correct")
        (`TextRenderComponent.SetTextRenderColor` _entered_code_2 (make `Color` 0 255 0 255))
        (`PrimitiveComponent.SetMaterial` (`self.lampu`) 0 "/Game/KEYPAD-fix/glow_hijau.glow_hijau")
        (`KismetSystemLibrary.RetriggerableDelay` 1.0)
        (bind _output_get (set `PlayerController.bShowMouseCursor` true _returnvalue_2))
        (bind _output_get_2 (set `PlayerController.bEnableMouseOverEvents` _output_get _returnvalue_2))
        (set `PlayerController.bEnableClickEvents` _output_get_2 _returnvalue_2)
        (for _array_element (`self.buttons array`)
          (bind _askeyyyyyyangka (cast `/Game/KEYPAD-fix/keyyyyyyangka` (`ChildActorComponent.ChildActor` _array_element)))
          (`/Game/KEYPAD-fix/keyyyyyyangka.reset` _askeyyyyyyangka))
        (`PlayerController.SetViewTargetWithBlend` (`GameplayStatics.GetPlayerController` 0) (`ActorComponent.GetOwner` (`/Game/ThirdPerson/Blueprints/BP_contoh.FollowCamera` (cast `/Game/ThirdPerson/Blueprints/BP_contoh` (`GameplayStatics.GetPlayerPawn` 0) :!pure true))) 0.4 "VTBlend_Linear" 0.0 false)
        (`TextRenderComponent.K2_SetText` (`self.entered code`) "")
        (`WidgetBlueprintLibrary.SetInputMode_GameOnly` (`GameplayStatics.GetPlayerController` 0))
        (`ActorComponent.K2_DestroyComponent` (`self.Boxcollision`))
        (set `/Game/ThirdPerson/Blueprints/BP_contoh.Keypad Interact Actor` null (`self.player ref`)))
      (:`then_1`
        (set `self.canEnter` true)))
    (else
      ;;[1 1 1] passcode salah, berubah warna
      (`|ExecutionSequence`
        (:`then_0`
          (`TextRenderComponent.K2_SetText` _entered_code "Try again")
          (`TextRenderComponent.SetTextRenderColor` _entered_code (make `Color` 0 0 255 255))
          (`PrimitiveComponent.SetMaterial` (`self.keypad`) 2 "/Engine/BasicShapes/glow.glow")
          (`KismetSystemLibrary.RetriggerableDelay` 1.5)
          (bind _output_get_3 (set `PlayerController.bEnableMouseOverEvents` false _returnvalue))
          (set `PlayerController.bEnableClickEvents` _output_get_3 _returnvalue)
          (for _array_element_2 (`self.buttons array`)
            (bind _askeyyyyyyangka_2 (cast `/Game/KEYPAD-fix/keyyyyyyangka` (`ChildActorComponent.ChildActor` _array_element_2)))
            (`/Game/KEYPAD-fix/keyyyyyyangka.reset` _askeyyyyyyangka_2))
          (`self.Initiate`)
          (set `self.canEnter` true))
        (:`then_1`
          (set `self.canEnter` false))))))

(fn `UserConstructionScript`)